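; BP_GameMode is the game mode that owns the HUD and the win and lose screens for a fight involving the player and a troll enemy.
; BeginPlay creates W_HUD as Hub, whose health bars are bound to CharacterRef and TrollRef through SetPlayertoHub and SetEnemytoHub.
; Victory and GameOver clear all widgets, show their result view, and switch to UI-only input with a visible cursor.
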(event EventBeginPlay
  (bind _returnvalue (UserInterface|CreateWidget "/Game/Blueprints/UI/HUD/W_HUD.W_HUD_C"))
  (bind _output_get (Variables|Default|SetHub _returnvalue))
  (UserInterface|Viewport|AddtoViewport _output_get 0))

(event EventTick
  (params (DeltaSeconds :type Float%20%28single-precision%29)))

(event EventVictory
  (bind _returnvalue (Game|GetPlayerController 0))
  (Viewport|RemoveAllWidgets)
  (bind _returnvalue_2 (UserInterface|CreateWidget "/Game/Blueprints/UI/HUD/WinView/W_WinView.W_WinView_C"))
  (UserInterface|Viewport|AddtoViewport _returnvalue_2 0)
  (Input|SetInputModeUIOnly _returnvalue 0 "DoNotLock")
  (Variables|/Script/Engine.PlayerController|SetbShowMouseCursor _returnvalue true))

(event EventGameOver
  (bind _returnvalue (Game|GetPlayerController 0))
  (Viewport|RemoveAllWidgets)
  (bind _returnvalue_2 (UserInterface|CreateWidget "/Game/Blueprints/UI/HUD/LoseView/W_LoseView.W_LoseView_C"))
  (UserInterface|Viewport|AddtoViewport _returnvalue_2 0)
  (Input|SetInputModeUIOnly _returnvalue 0 "DoNotLock")
  (Variables|/Script/Engine.PlayerController|SetbShowMouseCursor _returnvalue true))

(event EventSetEnemytoHub
  (Utilities|IsValid (Variables|Default|GetHub)
    (:Is%20Valid
      (Class|BEnemyHealthBar|InitializeWidget (Variables|/Game/Blueprints/UI/HUD/W_HUD.W_HUD_C|GetW_EnemyHealthBar (Variables|Default|GetHub)) (Variables|Default|GetTrollRef)))))

(event EventSetPlayertoHub
  (Utilities|IsValid (Variables|Default|GetHub)
    (:Is%20Valid
      (Class|BHUDHealthBar|InitializeWidget (Variables|/Game/Blueprints/UI/HUD/W_HUD.W_HUD_C|Getw_PlayerHealthBar (Variables|Default|GetHub)) (Variables|Default|GetCharacterRef)))))

(fn ConstructionScript)